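; Goblin enemy for a side-view sprite game, with health, player detection and a reward of critical meter and random EXP on death.
; Tick updates alive state, health bar widget and walk animation, while damage events reduce health and destroy it.
; Capsule hits on the player only play an attack animation, and a detection volume sets a sight flag exposed by getter.
; Patrol endpoints are computed at BeginPlay; follow and sprite-flip logic is disconnected.
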(event `ControlRotation`
  ;[0.499 1 0.9701] Rotation Control
)

(event `self.ReceiveTick`
  (params (DeltaSeconds :type "Float (single-precision)"))
  ;[1 1 1] Event Tick
  (if true
    (`self.Walking`)
    (if (> (`self.Health`) 0.0)
      (set `self.IsAlive` true)
      (`self.HealthPercentage`)
      (else
        (set `self.IsAlive` false)))))

(event `FollowPlayer`
  ;[1 0.9399 0.5624] Follow Player
)

(event `self.ReceiveAnyDamage`
  (params (Damage :type "Float (single-precision)") (DamageType :type "DamageType Object Reference") (InstigatedBy :type "Controller Object Reference") (DamageCauser :type "Actor Object Reference"))
  (bind _playerref (`self.PlayerRef`))
  ;[1 0.05759 0.2684] Taking Damage
  (bind _output_get (set `self.Health` (`KismetMathLibrary.FClamp` (- (`self.Health`) Damage) 0.0 100.0)))
  (if (`self.IsAlive`)
    (`KismetSystemLibrary.PrintString` (`KismetStringLibrary.Concat_StrStr` "Goblin Health: " (`KismetStringLibrary.Conv_DoubleToString` _output_get)) true true (struct :`R` 1.0 :`G` 0.022775 :`B` 0.975773 :`A` 1.0))
    (else
      (set `self.HaveDied` true)
      (`self.K2_DestroyActor`)
      (if (`self.HaveDied`)
        (set `/Game/Blueprints/Character1.CriticalMeter` (`KismetMathLibrary.FClamp` (+ (`/Game/Blueprints/Character1.CriticalMeter` _playerref) 30.0) 0.0 90.0) _playerref)
        (set `/Game/Blueprints/Character1.EXP` (+ (`/Game/Blueprints/Character1.EXP` _playerref) (`KismetMathLibrary.Conv_IntToDouble` (`KismetMathLibrary.Conv_Int64ToInt` (`KismetMathLibrary.FCeil64` (`KismetMathLibrary.RandomFloatInRange` 50.0 70.0))))) _playerref)))))

(event `Walking`
  ;[0.8503 0.6008 1] Walking Animation Setup
  (if (!= (`MovementComponent.Velocity` (`self.CharacterMovement`)) (0.0 0.0 0.0))
    (`/Engine/EditorBlueprintResources/StandardMacros.DoOnce` false :!label _label
      (:`Completed`
        (`PaperZDAnimInstance.JumpToNode` (`PaperZDAnimationComponent.AnimInstance` (`self.AnimationComponent`)) "WalkNode" "None")
        (`KismetSystemLibrary.Delay` 1.0)
        (goto _label :!via `Reset`)))))

(event `self.CapsuleComponent.OnComponentHit`
  (params (HitComponent :type "PrimitiveComponent Object Reference") (OtherActor :type "Actor Object Reference") (OtherComp :type "PrimitiveComponent Object Reference") (NormalImpulse :type "Vector Structure") (Hit :type "HitResult Structure (by ref)"))
  ;[0.9692 1 0.152] Attack
  (cast `/Game/Blueprints/Character1` OtherActor)
  (if (`/Game/Blueprints/Character1.IsAlive` (`self.PlayerRef`))
    (`/Engine/EditorBlueprintResources/StandardMacros.DoOnce` false :!label _label_2
      (:`Completed`
        (`PaperZDAnimInstance.JumpToNode` (`PaperZDAnimationComponent.AnimInstance` (`self.AnimationComponent`)) "AttackNode" "None")
        (`KismetSystemLibrary.Delay` 1.0)
        (goto _label_2 :!via `Reset`)))))

(event `UpdatePatrolLocation`
  (bind _returnvalue_x (`KismetMathLibrary.BreakVector` (`SceneComponent.K2_GetComponentLocation` (`self.CapsuleComponent`))))
  (bind _returnvalue_x_2 (`KismetMathLibrary.BreakVector` (`SceneComponent.K2_GetComponentLocation` (`self.CapsuleComponent`))))
  ;[1 0.05805 0.8703] Patrol Locations
  (`/Engine/EditorBlueprintResources/StandardMacros.DoOnce` false
    (:`Completed`
      (`|ExecutionSequence`
        (:`then_0`
          (bind _output_get (set `self.Location A` (`KismetMathLibrary.MakeVector` (+ _returnvalue_x_2 (`self.GoblinPatrolRadius`)))))
          (`KismetSystemLibrary.PrintString` (`KismetStringLibrary.Conv_VectorToString` _output_get)))
        (:`then_1`
          (bind _output_get_2 (set `self.Location B` (`KismetMathLibrary.MakeVector` (- _returnvalue_x (`self.GoblinPatrolRadius`)))))
          (`KismetSystemLibrary.PrintString` (`KismetStringLibrary.Conv_VectorToString` _output_get_2)))))))

(event `self.DetectCollision.OnComponentBeginOverlap`
  (params (OverlappedComponent :type "PrimitiveComponent Object Reference") (OtherActor :type "Actor Object Reference") (OtherComp :type "PrimitiveComponent Object Reference") (OtherBodyIndex :type Integer) (bFromSweep :type Boolean) (SweepResult :type "HitResult Structure (by ref)"))
  ;[0.5406 1 0.5633] Seeing Player
  (cast `/Game/Blueprints/Character1` OtherActor)
  (set `self.IsSeeingPlayer` true))

(event `self.DetectCollision.OnComponentEndOverlap`
  (params (OverlappedComponent :type "PrimitiveComponent Object Reference") (OtherActor :type "Actor Object Reference") (OtherComp :type "PrimitiveComponent Object Reference") (OtherBodyIndex :type Integer))
  ;[0.5406 1 0.5633] Seeing Player
  (cast `/Game/Blueprints/Character1` OtherActor)
  (set `self.IsSeeingPlayer` false))

(event `self.ReceiveBeginPlay`
  ;[1 0.4247 0.7284] Character Referance
  (bind _ascharacter_1 (cast `/Game/Blueprints/Character1` (`GameplayStatics.GetPlayerCharacter` 0)))
  (set `self.PlayerRef` _ascharacter_1)
  (`self.UpdatePatrolLocation`))

(fn `GetHaveDied`
  (returns (HaveDied :type Boolean))
  (return (`self.HaveDied`)))

(fn `GetIsSeeingPlayer`
  (returns (IsSeeingPlayer :type Boolean))
  (return (`self.IsSeeingPlayer`)))

(fn `HealthPercentage`
  (bind _asenemy_bars (cast `/Game/Blueprints/UI/EnemyBars` (`WidgetComponent.GetWidget` (`self.HealthBar`))))
  (`ProgressBar.SetPercent` (`/Game/Blueprints/UI/EnemyBars.Health` _asenemy_bars) (/ (`self.Health`) 100.0)))

(fn `UserConstructionScript`)